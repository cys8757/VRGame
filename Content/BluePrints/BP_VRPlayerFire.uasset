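; VR player component that provides right-hand aiming and firing for BP_VRPlayerPawn.
; Every tick, a line trace from the hand feeds the pawn's Niagara beam endpoints and moves its Niagara crosshair to the aim point, aligned to the last hit normal.
; Fire reuses that trace: on a hit it spawns an explosion and pushes physics-simulating components along the aim direction with mass-scaled, acceleration-change force.
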(event `self.ReceiveBeginPlay`
  (bind _asbp_vrplayer_pawn (cast `/Game/BluePrints/BP_VRPlayerPawn` (`self.GetOwner`)))
  (bind _output_get (set `self.me` _asbp_vrplayer_pawn))
  (set `self.hand` (`/Game/BluePrints/BP_VRPlayerPawn.Righthand` _output_get)))

(event `Fire`
  (bind _hit_component (`self.Hit Component`))
  (if (`self.bHit`)
    (`GameplayStatics.SpawnEmitterAtLocation` "/Game/StarterContent/Particles/P_Explosion.P_Explosion" (`self.end`))
    (if (`SceneComponent.IsSimulatingPhysics` _hit_component "None")
      (`PrimitiveComponent.AddForce` _hit_component (* (* (`KismetMathLibrary.Normal` (- (`self.end`) (`self.start`))) (`PrimitiveComponent.GetMass` _hit_component)) (`self.fireforce`)) "None" true))))

(event `self.ReceiveTick`
  (params (DeltaSeconds :type "Float (single-precision)"))
  (`self.DrawLine`))

(fn `DrawLine`
  (locals (LocalNormalVar :type "Vector Structure" :default (0.0 0.0 0.0)))
  (bind _hand (`self.hand`))
  (bind _returnvalue (`SceneComponent.K2_GetComponentLocation` _hand))
  (bind _firecrosshairniagarasystem (`/Game/BluePrints/BP_VRPlayerPawn.FireCrossHairNiagaraSystem` (`self.me`)))
  (`|ExecutionSequence`
    (:`then_0`
      (bind _output_get (set `self.start` _returnvalue))
      (bind _output_get_2 (set `self.end` (+ _returnvalue (* (`SceneComponent.GetForwardVector` _hand) (`self.lineDistance`)))))
      (bind (_outhit _returnvalue_2) (`KismetSystemLibrary.LineTraceSingleForObjects` _output_get _output_get_2 (`|MakeArray` "ObjectTypeQuery1" "ObjectTypeQuery2" "ObjectTypeQuery4" :!type "EObjectTypeQuery Enum") false (`|MakeArray` (`self.me`) :!type "Actor Object Reference") "None" true (struct :`R` 1.0 :`A` 1.0) (struct :`G` 1.0 :`A` 1.0) 0.5))
      (bind _output_get_3 (set `self.bHit` _returnvalue_2))
      (if _output_get_3
        (bind (_bblockinghit _binitialoverlap _time _distance _location _impactpoint _normal _impactnormal _physmat _hitactor _hitcomponent) (`GameplayStatics.BreakHitResult` _outhit))
        (set `self.end` _impactpoint)
        (set `self.Hit Actor` _hitactor)
        (set `local.LocalNormalVar` _impactnormal)
        (set `self.Hit Component` _hitcomponent)))
    (:`then_1`
      (`NiagaraDataInterfaceArrayFunctionLibrary.SetNiagaraArrayVector` (`/Game/BluePrints/BP_VRPlayerPawn.FireTraceNiagaraSystem` (`self.me`)) "User.PointArray" (`|MakeArray` (`self.start`) (`self.end`)))
      (`SceneComponent.K2_SetWorldLocationAndRotation` _firecrosshairniagarasystem (`self.end`) (`KismetMathLibrary.MakeRotFromZX` (`local.LocalNormalVar`) (`SceneComponent.GetForwardVector` _firecrosshairniagarasystem)) false false))))