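; Grab component for the VR player pawn that lets the right hand pick up and throw physics objects.
; On grab, a line trace forward from the hand finds a physics body, disables its physics and gravity, and attaches its actor to the hand.
; On release, it detaches, restores physics and adds the motion controller's linear velocity, scaled by a force multiplier, plus its angular velocity.
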(event `self.ReceiveBeginPlay`
  (bind _asbp_vrplayer_pawn (cast `/Game/BluePrints/BP_VRPlayerPawn` (`self.GetOwner`)))
  (bind _output_get (set `self.me` _asbp_vrplayer_pawn))
  (set `self.hand` (`/Game/BluePrints/BP_VRPlayerPawn.Righthand` _output_get))
  (set `self.controller` (`/Game/BluePrints/BP_VRPlayerPawn.RightMotionController` _output_get)))

(event `GrabPressed`
  (bind _hand (`self.hand`))
  (bind _hit_component (`self.Hit Component`))
  (bind _returnvalue (`SceneComponent.K2_GetComponentLocation` _hand))
  (bind (_outhit _returnvalue_2) (`KismetSystemLibrary.LineTraceSingleForObjects` _returnvalue (+ _returnvalue (* (`SceneComponent.GetForwardVector` _hand) (`self.LineDistance`))) (`|MakeArray` "ObjectTypeQuery4" :!type "EObjectTypeQuery Enum") false (`|MakeArray` (`self.me`) :!type "Actor Object Reference")))
  (bind _output_get (set `self.bHit` _returnvalue_2))
  (if _output_get
    (bind (_bblockinghit _binitialoverlap _time _distance _location _impactpoint _normal _impactnormal _physmat _hitactor _hitcomponent) (`GameplayStatics.BreakHitResult` _outhit))
    (set `self.Hit Component` _hitcomponent)
    (set `self.Hit Actor` _hitactor)
    (`PrimitiveComponent.SetSimulatePhysics` _hit_component false)
    (`PrimitiveComponent.SetEnableGravity` _hit_component false)
    (`Actor.K2_AttachToComponent` (`self.Hit Actor`) (`self.hand`) "None" "SnapToTarget" "KeepWorld" "KeepWorld" true)))

(event `GrabReleased`
  (bind _hit_component (`self.Hit Component`))
  (if (`self.bHit`)
    (`Actor.K2_DetachFromActor` (`self.Hit Actor`) "KeepWorld" "KeepWorld" "KeepWorld")
    (set `self.bHit` false)
    (`PrimitiveComponent.SetSimulatePhysics` _hit_component true)
    (`PrimitiveComponent.SetEnableGravity` _hit_component true)
    (bind _returnvalue (`PrimitiveComponent.GetPhysicsLinearVelocity` (`self.controller`) "None"))
    (`PrimitiveComponent.SetPhysicsLinearVelocity` (`self.Hit Component`) (* _returnvalue (`self.force`)) true "None")
    (`PrimitiveComponent.SetPhysicsAngularVelocityInDegrees` (`self.Hit Component`) (`PrimitiveComponent.GetPhysicsAngularVelocityInDegrees` (`self.controller`) "None") true "None")))