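; BP_VRPlayerMoveComp is a movement component that moves and turns the VR player that owns it.
; It caches the owner at BeginPlay, then feeds LeftX and LeftY axes into a shared Translate function along the actor's right and forward vectors.
; RightX applies smooth world yaw rotation.
; Both motions scale by speed and frame delta time, and translation sets location directly without sweep, so it ignores collision.
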(event `LeftX`
  (params (AxisValue :type "Float (double-precision)"))
  (`self.Translate` (`Actor.GetActorRightVector` (`self.me`)) AxisValue))

(event `LeftY`
  (params (AxisValue :type "Float (double-precision)"))
  (`self.Translate` (`Actor.GetActorForwardVector` (`self.me`)) AxisValue))

(event `RightX`
  (params (AxisValue :type "Float (double-precision)"))
  (`Actor.K2_AddActorWorldRotation` (`self.me`) (`KismetMathLibrary.MakeRotator` 0.0 0.0 (* AxisValue (`GameplayStatics.GetWorldDeltaSeconds`) (`self.rotSpeed`))) false false))

(event `self.ReceiveBeginPlay`
  ;[1 1 1] Cache 자주 사용하는 정보를 변수에 담아놓고 사용하면, 최적화에 좋다.
  (set `self.me` (`self.GetOwner`)))

(fn `Translate`
  (params (direction :type "Vector Structure") (`Axis Value` :type "Float (double-precision)"))
  (bind _me (`self.me`))
  (`Actor.K2_SetActorLocation` _me (+ (`Actor.K2_GetActorLocation` _me) (* (* direction (* `Axis Value` (`self.moveSpeed`))) (`GameplayStatics.GetWorldDeltaSeconds`))) false false))